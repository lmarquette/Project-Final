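; Paper2D boss enemy with health-threshold attacks, still partly built.
; Tick fires bullets from Arrow1 through a 0.2-second Delay and spawns a tentacle every frame at or below 75% health; lower-health branches are empty.
; Death sets the state and destroys the actor after a short delay.
; State-based flipbook updates and velocity-based facing exist but are not wired to run, and WallJump only performs a debug line trace.
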(event Custom|Wall%20Jump
  (bind _returnvalue (Transformation|GetActorLocation))
  ;[1 1 1] Maybe Reuse for firing at MC
  (Collision|LineTraceByChannel _returnvalue (select (Variables|Default|GetbisMovingRight) (+ _returnvalue "200.000000,0.000000,50.000000" "") (+ _returnvalue "-200.000000,0.000000,50.000000")) "TraceTypeQuery1" false 0 "Persistent"))

(event Custom|Death
  ;[1 1 1] Death
  (Math|Float|CompareFloat (Variables|Default|GetBoss%20Health) 0.0
    (:==
      _)
    (:<
      _))
  (Variables|Default|SetBoss%20State "NewEnumerator6")
  (Utilities|FlowControl|Delay 0.2)
  (Actor|DestroyActor))

(event Custom|UpdateAnimation
  ;[1 1 1] Handle Animation
  (switch Utilities|FlowControl|Switch|SwitchonBoss (Variables|Default|GetBoss%20State)
    (:NewEnumerator0
      (Sprite|SetFlipbook (Variables|Default|GetSprite) (select (> (Math|Vector|VectorLength (Transformation|GetVelocity)) 0.0) "/Game/Final/Flipbook/FB_Flying_Enemy.FB_Flying_Enemy" "/Game/Final/Flipbook/FB_Boss.FB_Boss")))
    (:NewEnumerator1
      (Sprite|SetFlipbook (Variables|Default|GetSprite) "/Game/Final/Flipbook/FB_Boss.FB_Boss"))
    (:NewEnumerator2
      (Sprite|SetFlipbook (Variables|Default|GetSprite) "/Game/Final/Flipbook/FB_Boss.FB_Boss"))
    (:NewEnumerator3
      (Sprite|SetFlipbook (Variables|Default|GetSprite) "/Game/Final/Flipbook/FB_Boss.FB_Boss"))
    (:NewEnumerator4
      (Sprite|SetFlipbook (Variables|Default|GetSprite)))
    (:NewEnumerator5
      (Sprite|SetFlipbook (Variables|Default|GetSprite)))
    (:NewEnumerator6
      (Sprite|SetFlipbook (Variables|Default|GetSprite)))))

(event EventTick
  (params (DeltaSeconds :type Float%20%28single-precision%29))
  (bind _returnvalue (Transformation|GetActorLocation))
  (bind _arrow1 (Variables|Default|GetArrow1))
  (bind _boss_health (Variables|Default|GetBoss%20Health))
  ;[1 1 1] Tick - Updates animation
  (Utilities|FlowControl|Sequence
    (:then_0
      (Utilities|FlowControl|Delay 0.2)
      (Game|SpawnActorfromClass "/Game/Final/Projectiles/BP_Enemy_Bullet.BP_Enemy_Bullet_C" (Math|Transform|MakeTransform (Transformation|GetWorldLocation _arrow1) (Transformation|GetWorldRotation _arrow1) "0.500000,0.500000,0.500000") "Undefined" 0 0))
    (:then_1
      (if (<= _boss_health 0.75)
        (Game|SpawnActorfromClass "/Game/Final/Blueprint/BP_Boss_Tentacle.BP_Boss_Tentacle_C" (Math|Transform|MakeTransform (Math|Vector|MakeVector (+ (.x _returnvalue) -1e+02) 0.0 (.z _returnvalue)) "0, 0, 0" "1,1,1") "Undefined" 0 0)))
    (:then_2
      (if (<= _boss_health 0.5)
        _))
    (:then_3
      (if (<= _boss_health 0.25)
        _))))

(event EventBeginPlay
  (Class|ActorComponent|SetIsReplicated (Variables|Default|GetSprite) true)
  (Variables|Default|SetBoss%20Health 1.0))

(fn ConstructionScript)