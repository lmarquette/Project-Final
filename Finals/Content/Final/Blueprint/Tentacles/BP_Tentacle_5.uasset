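; BP_Tentacle_5 is a tentacle hazard that lowers the main character's health on contact.
; Two box triggers, Box and Box1, each subtract a fixed amount from MCHealth when BP_Maincharacter begins overlapping them.
; Each box has its own DoOnce, reset after a short delay as a hit cooldown.
; The cast follows the DoOnce, so any other overlapping actor leaves that box's gate closed with no reset.
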(event OnComponentBeginOverlap(Box1)
  (params (OverlappedComponent :type Primitive%20Component%20Object%20Reference) (OtherActor :type Actor%20Object%20Reference) (OtherComp :type Primitive%20Component%20Object%20Reference) (OtherBodyIndex :type Integer) (bFromSweep :type Boolean) (SweepResult :type Hit%20Result%20Structure%20%28by%20ref%29))
  (Utilities|FlowControl|DoOnce false :!label _label
    (:Completed
      (bind _asbp_maincharacter (Utilities|Casting|CastToBP_Maincharacter OtherActor))
      (Variables|/Game/Final/Blueprint/BP_Maincharacter.BP_Maincharacter_C|SetMC_Health _asbp_maincharacter (- (Variables|/Game/Final/Blueprint/BP_Maincharacter.BP_Maincharacter_C|GetMC_Health _asbp_maincharacter) 0.2))
      (Utilities|FlowControl|Delay 1.0)
      (goto _label Reset))))

(event OnComponentBeginOverlap(Box)
  (params (OverlappedComponent :type Primitive%20Component%20Object%20Reference) (OtherActor :type Actor%20Object%20Reference) (OtherComp :type Primitive%20Component%20Object%20Reference) (OtherBodyIndex :type Integer) (bFromSweep :type Boolean) (SweepResult :type Hit%20Result%20Structure%20%28by%20ref%29))
  (Utilities|FlowControl|DoOnce false :!label _label
    (:Completed
      (bind _asbp_maincharacter (Utilities|Casting|CastToBP_Maincharacter OtherActor))
      (Variables|/Game/Final/Blueprint/BP_Maincharacter.BP_Maincharacter_C|SetMC_Health _asbp_maincharacter (- (Variables|/Game/Final/Blueprint/BP_Maincharacter.BP_Maincharacter_C|GetMC_Health _asbp_maincharacter) 0.2))
      (Utilities|FlowControl|Delay 1.0)
      (goto _label Reset))))

(event EventBeginPlay)

(event Collision|EventActorBeginOverlap
  (params (OtherActor :type Actor%20Object%20Reference)))

(event EventTick
  (params (DeltaSeconds :type Float%20%28single-precision%29)))

(fn ConstructionScript)