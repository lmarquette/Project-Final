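; The boss's second weak point, which tracks its own health and can fire a final laser attack.
; BeginPlay sets health, replicates the sprite and adds a boss health widget to the viewport.
; Tick polls health; at zero or below, it clears WeakPoint2 on the first BP_Boss found and destroys itself.
; FinalAttack spawns BP_Boss_Laser at an arrow; flipbook and facing logic is disconnected, and WallJump only draws a debug trace.
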(event Custom|Wall%20Jump
  (bind _returnvalue (Transformation|GetActorLocation))
  ;[1 1 1] Maybe Reuse for firing at MC
  (Collision|LineTraceByChannel _returnvalue (select (Variables|Default|GetbisMovingRight) (+ _returnvalue "200.000000,0.000000,50.000000" "") (+ _returnvalue "-200.000000,0.000000,50.000000")) "TraceTypeQuery1" false 0 "Persistent"))

(event Custom|Death
  ;[1 1 1] Death
  (Math|Float|CompareFloat (Variables|Default|GetWP%202%20Health) 0.0
    (:==
      _)
    (:<
      _))
  (bind _outactors (Actor|GetAllActorsOfClass "/Game/Final/Blueprint/Boss/BP_Boss.BP_Boss_C"))
  (bind _asbp_boss (Utilities|Casting|CastToBP_Boss (Utilities|Array|Get(acopy) _outactors)))
  (Variables|/Game/Final/Blueprint/Boss/BP_Boss.BP_Boss_C|SetWeak%20Point%202 _asbp_boss false)
  (Actor|DestroyActor))

(event Custom|UpdateAnimation
  ;[1 1 1] Handle Animation
  (switch Utilities|FlowControl|Switch|SwitchonBossWeakPoint (Variables|Default|GetBoss%20State)
    (:NewEnumerator0
      (Sprite|SetFlipbook (Variables|Default|GetSprite) (select (> (Math|Vector|VectorLength (Transformation|GetVelocity)) 0.0) "/Game/Final/Flipbook/FB_Flying_Enemy.FB_Flying_Enemy" "/Game/Final/Flipbook/FB_Boss.FB_Boss")))
    (:NewEnumerator1
      (Sprite|SetFlipbook (Variables|Default|GetSprite) "/Game/Final/Flipbook/FB_Boss.FB_Boss"))
    (:NewEnumerator2
      (Sprite|SetFlipbook (Variables|Default|GetSprite) "/Game/Final/Flipbook/FB_Boss.FB_Boss"))))

(event Custom|Final%20Attack
  ;[1 1 1] Final Attack
  (Game|SpawnActorfromClass "/Game/Final/Blueprint/Boss/BP_Boss_Laser.BP_Boss_Laser_C" (Transformation|GetWorldTransform (Variables|Default|GetFinal%20Attack%20Arrow)) "Undefined" 0 0))

(event EventTick
  (params (DeltaSeconds :type Float%20%28single-precision%29))
  ;[1 1 1] Tick - Updates animation
  (Utilities|FlowControl|Sequence
    (:then_0
      (CallFunction|Death))))

(event EventBeginPlay
  ;[1 1 1] Spawn
  (Class|ActorComponent|SetIsReplicated (Variables|Default|GetSprite) true)
  (Variables|Default|SetWP%202%20Health 1.0)
  (bind _returnvalue (UserInterface|CreateWidget "/Game/Final/Widget/W_BossHealth.W_BossHealth_C"))
  (UserInterface|Viewport|AddtoViewport _returnvalue 0))

(fn ConstructionScript)