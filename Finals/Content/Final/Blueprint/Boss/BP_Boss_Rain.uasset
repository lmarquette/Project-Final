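; BP_Boss_Rain is a short-lived spawner actor for a boss's rain attack.
; Tick feeds a one-second Delay, after which it spawns a BP_Boss_Rain_Bullet at the world transform of each of its five Arrow components.
; The actor then destroys itself, so the Tick-driven sequence acts as a one-shot delayed volley.
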(event EventBeginPlay)

(event Collision|EventActorBeginOverlap
  (params (OtherActor :type Actor%20Object%20Reference)))

(event EventTick
  (params (DeltaSeconds :type Float%20%28single-precision%29))
  (Utilities|FlowControl|Delay 1.0)
  (for _array_element (Utilities|Array|MakeArray (Variables|Default|GetArrow) (Variables|Default|GetArrow1) (Variables|Default|GetArrow2) (Variables|Default|GetArrow3) (Variables|Default|GetArrow4))
    (Game|SpawnActorfromClass "/Game/Final/Blueprint/Boss/BP_Boss_Rain_Bullet.BP_Boss_Rain_Bullet_C" (Transformation|GetWorldTransform _array_element) "Undefined" 0 0))
  (Actor|DestroyActor))

(fn ConstructionScript)