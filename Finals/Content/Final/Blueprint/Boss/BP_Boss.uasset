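; Paper2D boss that shows a health widget on spawn and escalates its attacks as BossHealth drops, destroying itself at zero.
; Tick drives everything: Delay-throttled bullets at random heights, a one-time tentacle at 75%, delayed rain projectiles from 50%, and a one-time laser at 10%.
; Arrow components position the bullet, rain and laser spawns.
; Flipbook state switching and facing logic exist but are disconnected; WallJump is a leftover debug trace.
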(event Custom|Wall%20Jump
  (bind _returnvalue (Transformation|GetActorLocation))
  ;[1 1 1] Maybe Reuse for firing at MC
  (Collision|LineTraceByChannel _returnvalue (select (Variables|Default|GetbisMovingRight) (+ _returnvalue "200.000000,0.000000,50.000000" "") (+ _returnvalue "-200.000000,0.000000,50.000000")) "TraceTypeQuery1" false 0 "Persistent"))

(event Custom|Death
  ;[1 1 1] Death
  (Math|Float|CompareFloat (Variables|Default|GetBoss%20Health) 0.0
    (:==
      _)
    (:<
      _))
  (Actor|DestroyActor))

(event Custom|UpdateAnimation
  ;[1 1 1] Handle Animation
  (switch Utilities|FlowControl|Switch|SwitchonBoss (Variables|Default|GetBoss%20State)
    (:NewEnumerator0
      (Sprite|SetFlipbook (Variables|Default|GetSprite) (select (> (Math|Vector|VectorLength (Transformation|GetVelocity)) 0.0) "/Game/Final/Flipbook/FB_Flying_Enemy.FB_Flying_Enemy" "/Game/Final/Flipbook/FB_Boss.FB_Boss")))
    (:NewEnumerator1
      (Sprite|SetFlipbook (Variables|Default|GetSprite) "/Game/Final/Flipbook/FB_Boss.FB_Boss"))
    (:NewEnumerator2
      (Sprite|SetFlipbook (Variables|Default|GetSprite) "/Game/Final/Flipbook/FB_Boss.FB_Boss"))
    (:NewEnumerator3
      (Sprite|SetFlipbook (Variables|Default|GetSprite) "/Game/Final/Flipbook/FB_Boss.FB_Boss"))
    (:NewEnumerator4
      (Sprite|SetFlipbook (Variables|Default|GetSprite)))
    (:NewEnumerator5
      (Sprite|SetFlipbook (Variables|Default|GetSprite)))
    (:NewEnumerator6
      (Sprite|SetFlipbook (Variables|Default|GetSprite)))))

(event Custom|Spawn%20Tentacle
  (bind _returnvalue (Transformation|GetActorLocation))
  ;[1 1 1] Spawn Tentacles
  (Utilities|FlowControl|DoOnce false
    (:Completed
      (Game|SpawnActorfromClass "/Game/Final/Blueprint/Boss/BP_Boss_Tentacle.BP_Boss_Tentacle_C" (Math|Transform|MakeTransform (Math|Vector|MakeVector (+ (.x _returnvalue) -5e+02) -1.0 (.z _returnvalue)) "0, 0, 0" "1,1,1") "AlwaysSpawn" 0 0))))

(event Custom|Air%20Rain%20Barrage%20Attack
  (bind _arrow2 (Variables|Default|GetArrow2))
  (bind _returnvalue (Transformation|GetWorldLocation _arrow2))
  ;[1 1 1] Air Attack
  (Utilities|FlowControl|Delay 1.0)
  (Game|SpawnActorfromClass "/Game/Final/Blueprint/Boss/BP_Boss_Rain.BP_Boss_Rain_C" (Math|Transform|MakeTransform (Math|Vector|MakeVector (+ (.x _returnvalue) (Math|Random|RandomFloatinRange -5e+02 0.0)) (.y _returnvalue) (.z _returnvalue)) (Transformation|GetWorldRotation _arrow2) "1,1,1") "Undefined" 0 0))

(event Custom|Basic%20Attack
  (bind _arrow1 (Variables|Default|GetArrow1))
  (bind _returnvalue (Transformation|GetWorldLocation _arrow1))
  ;[1 1 1] Basic Attack
  (Utilities|FlowControl|Delay 0.5)
  (Game|SpawnActorfromClass "/Game/Final/Blueprint/BP_Enemy_Bullet.BP_Enemy_Bullet_C" (Math|Transform|MakeTransform (Math|Vector|MakeVector (.x _returnvalue) (.y _returnvalue) (+ (.z _returnvalue) (Math|Random|RandomFloatinRange -1.5e+02 1.5e+02))) (Transformation|GetWorldRotation _arrow1) "0.500000,0.500000,0.500000") "Undefined" 0 0))

(event Custom|Final%20Attack
  ;[1 1 1] Final Attack
  (Game|SpawnActorfromClass "/Game/Final/Blueprint/Boss/BP_Boss_Laser.BP_Boss_Laser_C" (Transformation|GetWorldTransform (Variables|Default|GetFinal%20Attack%20Arrow)) "Undefined" 0 0))

(event EventTick
  (params (DeltaSeconds :type Float%20%28single-precision%29))
  (bind _boss_health (Variables|Default|GetBoss%20Health))
  ;[1 1 1] Tick - Updates animation
  (Utilities|FlowControl|Sequence
    (:then_0
      (CallFunction|Death))
    (:then_1
      (CallFunction|BasicAttack))
    (:then_2
      (if (<= _boss_health 0.75)
        (CallFunction|SpawnTentacle)))
    (:then_3
      (if (<= _boss_health 0.5)
        (CallFunction|AirRainBarrageAttack)))
    (:then_4
      (if (<= _boss_health 0.1)
        (Utilities|FlowControl|DoOnce false
          (:Completed
            (CallFunction|FinalAttack)))))))

(event EventBeginPlay
  ;[1 1 1] Spawn
  (Class|ActorComponent|SetIsReplicated (Variables|Default|GetSprite) true)
  (Variables|Default|SetBoss%20Health 1.0)
  (bind _returnvalue (UserInterface|CreateWidget "/Game/Final/Widget/W_BossHealth.W_BossHealth_C"))
  (UserInterface|Viewport|AddtoViewport _returnvalue 0))

(fn ConstructionScript)