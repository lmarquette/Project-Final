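; BP_Following_Boss is a flipbook-sprite boss that advances steadily along world +X and hurts the main character on contact.
; Tick drives the movement and aligns rotation to Arrow1 while the player cast succeeds, without tracking the player's position.
; Box overlap subtracts from MCHealth and launches the player forward and up.
; Death logic is a stub with unconnected destroy nodes, and UpdateAnimation is never called here.
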(event OnComponentBeginOverlap(Box)
  (params (OverlappedComponent :type Primitive%20Component%20Object%20Reference) (OtherActor :type Actor%20Object%20Reference) (OtherComp :type Primitive%20Component%20Object%20Reference) (OtherBodyIndex :type Integer) (bFromSweep :type Boolean) (SweepResult :type Hit%20Result%20Structure%20%28by%20ref%29))
  (bind _asbp_maincharacter (Utilities|Casting|CastToBP_Maincharacter OtherActor))
  (Variables|/Game/Final/Blueprint/BP_Maincharacter.BP_Maincharacter_C|SetMC_Health _asbp_maincharacter (- (Variables|/Game/Final/Blueprint/BP_Maincharacter.BP_Maincharacter_C|GetMC_Health _asbp_maincharacter) 0.3))
  (Character|LaunchCharacter _asbp_maincharacter "1000.000000,0.000000,1000.000000" false false))

(event Custom|Death
  ;[1 1 1] Death
  (Math|Float|CompareFloat 0.0 0.0))

(event Custom|UpdateAnimation
  ;[1 1 1] Handle Animation
  (switch Utilities|FlowControl|Switch|SwitchonFlyingEnemy "NewEnumerator0"
    (:NewEnumerator0
      (Sprite|SetFlipbook (Variables|Default|GetSprite) (select (> (Math|Vector|VectorLength (Transformation|GetVelocity)) 0.0) "/Game/Final/Flipbook/FB_Flying_Enemy.FB_Flying_Enemy" "/Game/Final/Flipbook/FB_Flying_Enemy.FB_Flying_Enemy")))
    (:NewEnumerator1
      (Sprite|SetFlipbook (Variables|Default|GetSprite) "/Game/Final/Flipbook/FB_Flying_Enemy.FB_Flying_Enemy"))
    (:NewEnumerator2
      (Sprite|SetFlipbook (Variables|Default|GetSprite) "/Game/Final/Flipbook/FB_MC.FB_MC"))))

(event EventTick
  (params (DeltaSeconds :type Float%20%28single-precision%29))
  ;[1 1 1] Tick - Updates animation
  (Utilities|Casting|CastToBP_Maincharacter (Game|GetPlayerCharacter 0))
  (Transformation|SetActorRotation (Transformation|GetWorldRotation (Variables|Default|GetArrow1)))
  (Pawn|Input|AddMovementInput "1.000000,0.000000, 0" 0.8 false))

(event EventBeginPlay
  (Class|ActorComponent|SetIsReplicated (Variables|Default|GetSprite) true))

(fn ConstructionScript)