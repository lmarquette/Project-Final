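; BP_RNG_Box is a gamble box that randomly heals or hurts the main character when stomped.
; On box overlap with a stomping BP_Maincharacter, a two-way random roll either adds health or subtracts some.
; The damage roll always explodes with sound and destroys the box.
; The heal roll caps health at full, and only plays smoke and sound and destroys the box when that cap is exceeded.
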(event OnComponentBeginOverlap(Box)
  (params (OverlappedComponent :type Primitive%20Component%20Object%20Reference) (OtherActor :type Actor%20Object%20Reference) (OtherComp :type Primitive%20Component%20Object%20Reference) (OtherBodyIndex :type Integer) (bFromSweep :type Boolean) (SweepResult :type Hit%20Result%20Structure%20%28by%20ref%29))
  (bind _returnvalue (Transformation|GetActorLocation))
  (bind _returnvalue_2 (Transformation|GetActorLocation))
  (bind _asbp_maincharacter (Utilities|Casting|CastToBP_Maincharacter OtherActor))
  (if (Variables|/Game/Final/Blueprint/BP_Maincharacter.BP_Maincharacter_C|GetStomping _asbp_maincharacter)
    (switch int (Math|Random|RandomIntegerinRange 0 1)
      (:0
        (Variables|/Game/Final/Blueprint/BP_Maincharacter.BP_Maincharacter_C|SetMC_Health _asbp_maincharacter (+ (Variables|/Game/Final/Blueprint/BP_Maincharacter.BP_Maincharacter_C|GetMC_Health _asbp_maincharacter) 1.0))
        (Math|Float|CompareFloat (Variables|/Game/Final/Blueprint/BP_Maincharacter.BP_Maincharacter_C|GetMC_Health _asbp_maincharacter) 1.0
          (:>
            (Variables|/Game/Final/Blueprint/BP_Maincharacter.BP_Maincharacter_C|SetMC_Health _asbp_maincharacter 1.0)
            (Effects|SpawnEmitteratLocation "/Game/StarterContent/Particles/P_Smoke.P_Smoke" _returnvalue_2 "0, 0, 0" "2.000000,2.000000,2.000000")
            (Audio|PlaySoundatLocation "/Game/StarterContent/Audio/Collapse02.Collapse02" _returnvalue_2 "0, 0, 0" 1.0 1.0 0.0 0 0 0)
            (Actor|DestroyActor))))
      (:1
        (Variables|/Game/Final/Blueprint/BP_Maincharacter.BP_Maincharacter_C|SetMC_Health _asbp_maincharacter (- (Variables|/Game/Final/Blueprint/BP_Maincharacter.BP_Maincharacter_C|GetMC_Health _asbp_maincharacter) 0.4))
        (Effects|SpawnEmitteratLocation "/Game/StarterContent/Particles/P_Explosion.P_Explosion" _returnvalue "0, 0, 0" "2.000000,2.000000,2.000000")
        (Audio|PlaySoundatLocation "/Game/StarterContent/Audio/Explosion02.Explosion02" _returnvalue "0, 0, 0" 1.0 1.0 0.0 0 0 0)
        (Actor|DestroyActor)))))

(event EventBeginPlay)

(event Collision|EventActorBeginOverlap
  (params (OtherActor :type Actor%20Object%20Reference)))

(event EventTick
  (params (DeltaSeconds :type Float%20%28single-precision%29)))

(fn ConstructionScript)