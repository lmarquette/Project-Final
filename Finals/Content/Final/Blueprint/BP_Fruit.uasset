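; BP_Fruit is a pickup that grants the player character the dash ability.
; Box overlap begin and end events toggle an IsSteppingOn flag, without checking which actor overlaps.
; Pressing Interact while the flag is set casts player 0's character to BP_Maincharacter and sets CanDash to true.
; The fruit stays in the world afterwards, and debug prints report overlap and pickup.
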(event OnComponentBeginOverlap(Box)
  (params (OverlappedComponent :type Primitive%20Component%20Object%20Reference) (OtherActor :type Actor%20Object%20Reference) (OtherComp :type Primitive%20Component%20Object%20Reference) (OtherBodyIndex :type Integer) (bFromSweep :type Boolean) (SweepResult :type Hit%20Result%20Structure%20%28by%20ref%29))
  (Variables|Default|Setis%20stepping%20on true)
  (Development|PrintString "stepping on fruit"))

(event OnComponentEndOverlap(Box)
  (params (OverlappedComponent :type Primitive%20Component%20Object%20Reference) (OtherActor :type Actor%20Object%20Reference) (OtherComp :type Primitive%20Component%20Object%20Reference) (OtherBodyIndex :type Integer))
  (Variables|Default|Setis%20stepping%20on false))

(event EventBeginPlay)

(event Collision|EventActorBeginOverlap
  (params (OtherActor :type Actor%20Object%20Reference)))

(event EventTick
  (params (DeltaSeconds :type Float%20%28single-precision%29)))

(event Input|ActionEvents|InputActionInteract
  (params (Key :type Key%20Structure))
  (:Pressed
    (if (Variables|Default|Getis%20stepping%20on)
      (bind _asbp_maincharacter (Utilities|Casting|CastToBP_Maincharacter (Game|GetPlayerCharacter 0)))
      (Variables|/Game/Final/Blueprint/BP_Maincharacter.BP_Maincharacter_C|Setcan_dash _asbp_maincharacter true)
      (Development|PrintString "picked up fruit"))))

(fn ConstructionScript)